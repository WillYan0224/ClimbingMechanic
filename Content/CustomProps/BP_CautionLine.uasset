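; BP_CautionLine is a caution-line prop that animates the material on its plane mesh by shifting the UV V offset.
; A looping two-second timer started at BeginPlay replays a timeline, which adds its value to the last saved row and writes UVOffsetV.
; Each update saves that sum as the next start, so the offset accumulates across cycles, and prints it for debugging.
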(event Custom|OnAdvance
  (Variables|Default|SetCurrentRow (Variables|Default|GetStartRow))
  (bind _v (Timeline|TL_ValueAnim PlayFromStart)
    (:Update
      (Rendering|Material|SetScalarParameterValueonMaterials (Variables|Default|GetSM_Plane) "UVOffsetV" (+ _v (Variables|Default|GetCurrentRow)))
      (Variables|Default|SetStartRow (+ _v (Variables|Default|GetCurrentRow)))
      (Development|PrintString (Utilities|String|ToString(Float) (+ _v (Variables|Default|GetCurrentRow))) true true "(R=0.000000,G=0.660000,B=1.000000,A=1.000000)" 2.0 "0"))))

(event EventBeginPlay
  (Utilities|Time|SetTimerbyEvent (delegate Custom|OnAdvance) 2.0 true)
  (bind _returnvalue (Rendering|Material|CreateDynamicMaterialInstance (Variables|Default|GetSM_Plane) 0 0 "None" :!class /Script/Engine.PrimitiveComponent))
  (Variables|Default|SetCreated_Dy_MI_CautionLine _returnvalue))

(fn ConstructionScript)